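; BP_HighJumper is an enemy Blueprint that gives visual feedback when it is highlighted as a possession target.
; On highlight, if CanBePossessed passes, it draws an outline on all its components through AOSACOutlineOverlay and activates its Niagara effect.
; On unhighlight, it disables all outlines and deactivates the effect.
; The graph holds no jump or other movement logic.
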(event `HighlightableInterface.OnHighlight`
  (if (`self.CanBePossessed`)
    (`AOSAC_OutlineOverlay.LvEnableOutlineOnActor` (`self.AOSAC_OutlineOverlay`) self "AllComps" true true (struct :`G` 81.743172 :`B` 100.0 :`A` 1.0))
    (`ActorComponent.SetActive` (`self.Niagara`) true false)))

(event `HighlightableInterface.OnUnhighlight`
  (`AOSAC_OutlineOverlay.LvDisableAllOutline` (`self.AOSAC_OutlineOverlay`))
  (`ActorComponent.SetActive` (`self.Niagara`) false false))

(fn `UserConstructionScript`)